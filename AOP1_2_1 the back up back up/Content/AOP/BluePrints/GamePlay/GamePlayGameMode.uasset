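; Gameplay game mode that gives the first joining player a Light character and every later player a Dark one.
; On a new player, it finds the start named Light or Dark, spawns the matching character there and possesses it, using a counter to switch sides.
; A ChoosePlayerStart function returns the first start whose tag is not None and retags it Taken, without skipping starts already marked Taken.
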(event Custom|Spawn%20and%20Possess
  (params (SpawnTransform :type Transform) (Owner :type Actor%20Object%20Reference) (Target :type Controller%20Object%20Reference))
  ;[1 1 1] Spawns and posses the character for the new starting player
  (if (== (Variables|Default|GetNum) 0)
    (bind _returnvalue (Game|SpawnActorfromClass "/Game/AOP/BluePrints/LightCharacter.LightCharacter_C" SpawnTransform "Undefined" Owner 0))
    (Pawn|Possess Target _returnvalue)
    (Variables|Default|SetNum 1)
    (else
      (bind _returnvalue_2 (Game|SpawnActorfromClass "/Game/AOP/BluePrints/DarkCharacter.DarkCharacter_C" SpawnTransform "Undefined" Owner "/Game/AOP/AI/Melee/Melee_Base.Melee_Base_C" 0))
      (Pawn|Possess Target _returnvalue_2))))

(event EventHandleStartingNewPlayer
  (params (NewPlayer :type Player%20Controller%20Object%20Reference))
  ;[1 1 1] Handles starting a new player
  (if (== (Variables|Default|GetNum) 0)
    (CallFunction|SpawnandPossess (Transformation|GetActorTransform (Class|GameModeBase|FindPlayerStart NewPlayer "Light")) NewPlayer NewPlayer)
    (else
      (CallFunction|SpawnandPossess (Transformation|GetActorTransform (Class|GameModeBase|FindPlayerStart NewPlayer "Dark")) NewPlayer NewPlayer))))

(fn ConstructionScript)

(fn ChoosePlayerStart
  (params (Player :type Controller%20Object%20Reference))
  (bind _outactors (Actor|GetAllActorsOfClass "/Script/Engine.PlayerStart"))
  (for _array_element _outactors
    (if (Utilities|Name|NotEqual(Name) (Variables|/Script/Engine.PlayerStart|GetPlayerStartTag _array_element) "None")
      (Variables|/Script/Engine.PlayerStart|SetPlayerStartTag _array_element "Taken")
      (return _array_element))))