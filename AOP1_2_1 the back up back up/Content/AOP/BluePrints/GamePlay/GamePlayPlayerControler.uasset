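; Gameplay player controller that holds server-side helpers for gold purchases and melee AI spawning, plus an event that sets the IsLight flag.
; BuyFromShop compares cost to current gold on authority, returning the updated gold and a CanSpawn flag.
; SpawnMelee takes a CanSpawn flag and, on authority, spawns an AI running MeleeBT at a hardcoded transform.
; Nothing here calls either function, and feedback is only debug prints.
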(event Custom|is%20light%20set?
  (params (Is%20Light :type Boolean))
  (Variables|Default|SetIs%20Light Is%20Light))

(event EventBeginPlay)

(event EventTick
  (params (DeltaSeconds :type Float%20%28single-precision%29)))

(fn ConstructionScript)

(fn BuyfromShop
  (params (Cost :type Integer) (Current%20Gold :type Integer))
  (bind _returnvalue (<= Cost Current%20Gold))
  (Networking|SwitchHasAuthority
    (:Authority
      (if _returnvalue
        (Development|PrintString "you have enough money ")
        (return (- Current%20Gold Cost) _returnvalue)
        (else
          (Development|PrintString "you do not  have enough money ")
          (return Current%20Gold _returnvalue))))))

(fn SpawnMelee
  (params (Can%20Spawn :type Boolean))
  (Networking|SwitchHasAuthority
    (:Authority
      (if Can%20Spawn
        (AI|SpawnAIFromClass 0 "/Game/AOP/AI/Melee/MeleeBT.MeleeBT" "1206.637085,913.940613,192.001297" "0,-90.000000, 0" false)
        (else
          (Development|PrintString "Not Enough Gold"))))))