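; Lobby game mode that overrides player start selection for joining players.
; ChoosePlayerStart returns the first PlayerStart with a tag other than None and retags it "Taken", which still passes that check, so the same start can be picked again.
; HandleStartingNewPlayer is an empty override; authority-only logic to spawn and possess a LightCharacter at a player start is disconnected and never runs.
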(event EventBeginPlay)

(event EventTick
  (params (DeltaSeconds :type Float%20%28single-precision%29)))

(event EventHandleStartingNewPlayer
  (params (NewPlayer :type Player%20Controller%20Object%20Reference)))

(fn ConstructionScript)

(fn ChoosePlayerStart
  (params (Player :type Controller%20Object%20Reference))
  (bind _outactors (Actor|GetAllActorsOfClass "/Script/Engine.PlayerStart"))
  (for _array_element _outactors
    (if (Utilities|Name|NotEqual(Name) (Variables|/Script/Engine.PlayerStart|GetPlayerStartTag _array_element) "None")
      (Variables|/Script/Engine.PlayerStart|SetPlayerStartTag _array_element "Taken")
      (return _array_element))))